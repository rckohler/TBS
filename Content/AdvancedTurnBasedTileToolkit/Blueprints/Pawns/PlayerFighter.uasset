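; PlayerFighter is a player pawn Blueprint for the Fighter class in the Advanced Turn Based Tile Toolkit.
; On BeginPlay it sets its MyClass struct to mark it as a Fighter rather than a Mage.
; It overrides the parent's AttackVictim and QAbility events, calling the parent logic and then printing debug strings as placeholders for custom behavior.
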(event EventBeginPlay
  (|CallParentFunction)
  (Variables|Default|SetMyClass (Utilities|Struct|MakeNewUserDefinedStruct true false)))

(event Collision|EventActorBeginOverlap
  (params (OtherActor :type Actor%20Object%20Reference)))

(event EventTick
  (params (DeltaSeconds :type Float%20%28single-precision%29))
  (|CallParentFunction 0.0))

(event EventAttackVictim
  (params (Victim :type Unit%20Parent%20Object%20Reference))
  (|CallParentFunction Victim)
  (Development|PrintString "Custom Attack"))

(event EventQAbility
  (|CallParentFunction)
  (Development|PrintString "Fighter Q"))

(fn ConstructionScript
  (|CallParentFunction))