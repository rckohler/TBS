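; Potion item for the 2D example game that acts on a hero unit when activated, then destroys itself and plays a potion sound.
; ActivateItem casts the activating unit to Unit_2D_Sprite_Hero, zeroes CurrentWounds and writes PercentFill on its dynamic health bar material.
; The capped HealAmount calculation is unused, and PercentFill comes from a literal zero-by-zero division.
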(event EventBeginPlay)

(event EventActorBeginOverlap
  (params (OtherActor :type Actor%20Object%20Reference)))

(event EventTick
  (params (DeltaSeconds :type Float%20%28single-precision%29)))

(event EventActivateItem
  (params (Activating%20Unit :type Unit%20Parent%202D%20Object%20Reference))
  (Utilities|Casting|CastToUnit_2D_Sprite_Hero Activating%20Unit)
  (Variables|/Game/AdvancedTurnBasedTileToolkit/Blueprints/Pawns/CustomContent/units/Unit_Parent.Unit_Parent_C|SetCurrentWounds Activating%20Unit 0)
  (Rendering|Material|SetScalarParameterValue (Variables|/Game/AdvancedTurnBasedTileToolkit/Blueprints/Pawns/CustomContent/units/Unit_Parent.Unit_Parent_C|GetDynamic%20Health%20Bar%20Material Activating%20Unit) "PercentFill" (/ 0.0 0.0) :!class /Script/Engine.MaterialInstanceDynamic)
  (Actor|DestroyActor)
  (Audio|PlaySound2D "/Game/AdvancedTurnBasedTileToolkit/Maps/2D_Game_Example/Sound/Potion.Potion"))

(fn ConstructionScript
  (|CallParentFunction))